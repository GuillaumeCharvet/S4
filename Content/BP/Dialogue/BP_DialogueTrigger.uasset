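; Box trigger volume that plays dialogue when the player walks into it.
; Construction runs the parent script, then sizes the box from BoxScale and lifts it by the Z extent so its base sits at the relative origin.
; While enabled, an overlap by the BP_Player capsule calls PlayDialogue with the player's MediaSound attenuation settings.
; IsSaidOnce disables the trigger after it plays.
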(event `self.ReceiveBeginPlay`)

(event `SetBoxScale`
  (bind (_boxscale_x _boxscale_y _boxscale_z) (`KismetMathLibrary.BreakVector` (`self.BoxScale`)))
  (`BoxComponent.SetBoxExtent` (`self.TriggerBox`) (`self.BoxScale`) true)
  (`SceneComponent.K2_SetRelativeLocation` (`self.TriggerBox`) (`KismetMathLibrary.MakeVector` 0.0 0.0 _boxscale_z) false false))

(event `self.TriggerBox.OnComponentBeginOverlap`
  (params (OverlappedComponent :type "PrimitiveComponent Object Reference") (OtherActor :type "Actor Object Reference") (OtherComp :type "PrimitiveComponent Object Reference") (OtherBodyIndex :type Integer) (bFromSweep :type Boolean) (SweepResult :type "HitResult Structure (by ref)"))
  (bind _asbp_player (cast `/Game/BP/Character/BP_Player` OtherActor))
  (if (== OtherComp (`Character.CapsuleComponent` _asbp_player))
    (if (`self.IsEnabled`)
      (`self.PlayDialogue` (`SynthComponent.AttenuationSettings` (`/Game/BP/Character/BP_Player.MediaSound` _asbp_player)))
      (if (`self.IsSaidOnce`)
        (set `self.IsEnabled` false)))))

(fn `UserConstructionScript`
  (`parent.UserConstructionScript`)
  (`self.SetBoxScale`))