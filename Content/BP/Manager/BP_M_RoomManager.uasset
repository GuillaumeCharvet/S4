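; Room manager Blueprint that tracks, spawns and destroys the level's rooms.
; On BeginPlay it fills AllRooms with every existing BPA_RoomParent actor.
; CreateRoom spawns a given room class at the world location and rotation of an exit, passing the new room a manager reference and its opposite room.
; CreateRoom and DestroyRoom keep AllRooms in sync as rooms are added or removed.
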(event `self.ReceiveBeginPlay`
  (bind _outactors (`GameplayStatics.GetAllActorsOfClass` "/Game/BP/Rooms/BPA_RoomParent.BPA_RoomParent_C"))
  (set `self.AllRooms` _outactors))

(event `CreateRoom`
  (params (TypeOfRoom :type "/Game/BP/Rooms/BPA_RoomParent Class Reference") (ExitToConnect :type "/Game/BP/Components/SceneComponents/BP_SC_RoomConnexion Object Reference") (OppositeRoom :type "/Game/BP/Rooms/BPA_RoomParent Object Reference"))
  (bind _returnvalue (`|SpawnActorFromClass` TypeOfRoom (`KismetMathLibrary.MakeTransform` (`SceneComponent.K2_GetComponentLocation` ExitToConnect) (`SceneComponent.K2_GetComponentRotation` ExitToConnect)) "Undefined" "OverrideRootScale" null self OppositeRoom null))
  (`KismetArrayLibrary.Array_Add` (`self.AllRooms`) _returnvalue))

(event `DestroyRoom`
  (params (RoomToDestroy :type "/Game/BP/Rooms/BPA_RoomParent Object Reference"))
  (`KismetArrayLibrary.Array_RemoveItem` (`self.AllRooms`) RoomToDestroy)
  (`self.K2_DestroyActor` RoomToDestroy))

(fn `UserConstructionScript`)