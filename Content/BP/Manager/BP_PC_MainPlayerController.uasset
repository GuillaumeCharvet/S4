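; Main player controller for a first-person game with a medicine-need meter, sleep-driven day progression and interactable objects.
; Creates the HUD, forwards movement and look input to the character while movement is allowed, and toggles a pause menu.
; A camera line trace on Tick selects interactive objects for use with E.
; A Tick-fed Delay raises medicine need about once a second and updates its bar; the post-process update is an empty stub.
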(event `self.ReceiveBeginPlay`
  ;[0.3986 1 0.1379] BeginPlay
  (`|ExecutionSequence`
    (:`then_0`
      ;;[1 1 1] Create UI
      (bind _returnvalue (`|CreateWidget` "/Game/BP/UI/WBP_MedicineNeeds.WBP_MedicineNeeds_C" self self))
      (bind _output_get (set `self.MedUI` _returnvalue))
      (`UserWidget.AddToViewport` _output_get 0)
      (bind _returnvalue_2 (`|CreateWidget` "/Game/BP/UI/WBP_InteractTo.WBP_InteractTo_C" self))
      (bind _output_get_2 (set `self.InteractUI` _returnvalue_2))
      (`UserWidget.AddToViewport` _output_get_2 0))
    (:`then_1`
      ;;[1 1 1] Getters
      (bind _returnvalue_3 (`GameplayStatics.GetActorOfClass` "/Script/Engine.PostProcessVolume"))
      (set `self.PostProcVol` _returnvalue_3)
      (set `self.Player Character` (`/Game/BP/FunctionLibraries/BP_FL_Getters.GetMyCharacter`)))))

(event `self.ReceiveTick`
  (params (DeltaSeconds :type "Float (single-precision)"))
  ;[0 0.3464 1] EventTick
  (`|ExecutionSequence`
    (:`then_0`
      (if (`self.HasToRaycast`)
        (`self.RaycastThings`)))
    (:`then_2`
      (`self.CustomTick`))))

(event `Sleep`
  (set `self.CanMove` false)
  (bind _result (`/Engine/EditorBlueprintResources/StandardMacros.IncrementInt` (`KismetMathLibrary.Conv_ByteToInt` (`self.CurrentDay`)))
    (:`  `
      (set `self.CurrentDay` (cast `/Game/BP/Enum/BP_E_Days` (`KismetMathLibrary.Conv_IntToByte` _result)))
      (set `self.HasTakenMedicine` false)
      (set `/Game/BP/Character/BP_Player.ClosingEyes` true (`self.Player Character`)))))

(event `CustomTick`
  (`KismetSystemLibrary.Delay` 1.0)
  (`self.MedicineChrono`))

(event `Pause/Unpause Game`
  (bind _returnvalue (`GameplayStatics.GetPlayerController` 0))
  (`/Engine/EditorBlueprintResources/StandardMacros.FlipFlop`
    (:`A`
      (`WidgetBlueprintLibrary.SetInputMode_UIOnlyEx` _returnvalue (stale _returnvalue_2))
      (bind _returnvalue_2 (`|CreateWidget` "/Game/BP/UI/WBP_PauseMenu.WBP_PauseMenu_C"))
      (`UserWidget.AddToViewport` _returnvalue_2 0)
      (`GameplayStatics.SetGamePaused` true)
      (set `self.bShowMouseCursor` true))
    (:`B`
      (`WidgetBlueprintLibrary.SetInputMode_GameOnly` _returnvalue)
      (`WidgetLayoutLibrary.RemoveAllWidgets`)
      (`GameplayStatics.SetGamePaused` false)
      (set `self.bShowMouseCursor` false))))

(event `MedicineChrono`
  (set `self.MedicineNeeds` (`KismetMathLibrary.Clamp` (+ (`self.MedicineNeeds`) 1) 0 100))
  (`/Game/BP/UI/WBP_MedicineNeeds.UpdateBar` (`self.MedUI`))
  (`self.UpdatePostProcMedic`))

(event `UpdatePostProcMedic`
  ;[1 0 0] PostProcessManip
)

(event `Key|P` :paused true
  (params (Key :type "Key Structure"))
  (:`Pressed`
    (`self.Pause/Unpause Game`)))

(event `Key|E`
  (params (Key :type "Key Structure"))
  (:`Pressed`
    (if (`self.CanMove`)
      (`/Engine/EditorBlueprintResources/StandardMacros.IsValid` (`self.SelectedObject`)
        (:`Is Valid`
          (`/Game/BP/Abstract/BP_Interactive.Interaction` (`self.SelectedObject`)))))))

(event `InputAxis|Turn` :overrideparent false
  (params (AxisValue :type "Float (single-precision)"))
  (if (`self.CanMove`)
    (`/Game/BP/Character/BP_Player.AxisTurn` (`self.Player Character`) AxisValue)))

(event `InputAxis|LookUp` :overrideparent false
  (params (AxisValue :type "Float (single-precision)"))
  (if (`self.CanMove`)
    (`/Game/BP/Character/BP_Player.AxisLookUp` (`self.Player Character`) AxisValue)))

(event `InputAxis|MoveRight`
  (params (AxisValue :type "Float (single-precision)"))
  (if (`self.CanMove`)
    (`/Game/BP/Character/BP_Player.AxisMoveRIght` (`self.Player Character`) AxisValue)))

(event `InputAxis|MoveForward`
  (params (AxisValue :type "Float (single-precision)"))
  (if (`self.CanMove`)
    (`/Game/BP/Character/BP_Player.AxisMoveForward` (`self.Player Character`) AxisValue)))

(event `InputAxis|LookUpRate`
  (params (AxisValue :type "Float (single-precision)"))
  (if (`self.CanMove`)
    (`/Game/BP/Character/BP_Player.AxisLookUpRate` (`self.Player Character`) AxisValue)))

(event `InputAxis|TurnRate`
  (params (AxisValue :type "Float (single-precision)"))
  (if (`self.CanMove`)
    (`/Game/BP/Character/BP_Player.AxisTurnRate` (`self.Player Character`) AxisValue)))

(fn `RaycastThings`
  (bind _firstpersoncamera (`/Game/BP/Character/BP_Player.FirstPersonCamera` (`self.Player Character`)))
  (bind _returnvalue (`SceneComponent.K2_GetComponentLocation` _firstpersoncamera))
  ;[0.3551 1 0.6655] Raycast
  (bind _outhit (`KismetSystemLibrary.LineTraceSingle` _returnvalue (+ _returnvalue (* (`SceneComponent.GetForwardVector` _firstpersoncamera) (`self.GrabDistance`))) "TraceTypeQuery1"))
  (bind (_bblockinghit _binitialoverlap _time _distance _location _impactpoint _normal _impactnormal _physmat _hitactor _hitcomponent) (`GameplayStatics.BreakHitResult` _outhit))
  ;[1 1 1] Raycast To Bp_Interactive
  (bind _asbp_interactive (cast `/Game/BP/Abstract/BP_Interactive` _hitactor)
    (:`then`
      ;;[0.5431 1 0.2257] Selection
      (if (== _hitcomponent (`/Game/BP/Abstract/BP_Interactive.InteractionBox` _asbp_interactive))
        (`/Engine/EditorBlueprintResources/StandardMacros.IsValid` (`self.SelectedObject`)
          (:`Is Not Valid`
            (bind _output_get (set `self.SelectedObject` _asbp_interactive))
            (`/Game/BP/Abstract/BP_Interactive.OnSelected` _output_get)))))
    (:`CastFailed`
      ;;[1 0.277 0.7133] Unselection
      (`/Engine/EditorBlueprintResources/StandardMacros.IsValid` (`self.SelectedObject`)
        (:`Is Valid`
          (`/Game/BP/Abstract/BP_Interactive.OnUnselected` (`self.SelectedObject`))
          (set `self.SelectedObject` null))))))

(fn `UserConstructionScript`)