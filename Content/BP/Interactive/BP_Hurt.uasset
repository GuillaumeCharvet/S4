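; BP_Hurt is an interactable hazard that injures the player and raises their need for medicine.
; Its Interaction event adds a fixed amount to MedicineNeeds on the main player controller (player 0) and refreshes the MedUI bar.
; It then destroys itself, prints an on-screen warning to take pills, and calls the parent Interaction.
; If the controller cast fails, none of this runs.
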(event `self.Interaction`
  (bind _asbp_pc_main_player_controller (cast `/Game/BP/Manager/BP_PC_MainPlayerController` (`GameplayStatics.GetPlayerController` 0)))
  (set `/Game/BP/Manager/BP_PC_MainPlayerController.MedicineNeeds` (+ (`/Game/BP/Manager/BP_PC_MainPlayerController.MedicineNeeds` _asbp_pc_main_player_controller) 90) _asbp_pc_main_player_controller)
  (`/Game/BP/UI/WBP_MedicineNeeds.UpdateBar` (`/Game/BP/Manager/BP_PC_MainPlayerController.MedUI` _asbp_pc_main_player_controller))
  (`self.K2_DestroyActor`)
  (`KismetSystemLibrary.PrintString` "Oof you hurt yourself. Quick, eat your pills." true true (struct :`R` 1.0 :`B` 0.075629 :`A` 1.0) 10.0)
  (`parent.Interaction`))

(fn `UserConstructionScript`
  (`parent.UserConstructionScript`))