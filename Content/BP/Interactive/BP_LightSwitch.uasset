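; BP_LightSwitch is an interactive switch that turns a set of lights on and off.
; Interaction calls SwitchOn or SwitchOff based on IsOn, and both act only when CanBeSwitched is true.
; Each toggles light component visibility across LightsToSwitch, updates IsOn, then copies that state to OtherSwitchesForSameLights so switches sharing the lights stay in sync.
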(event `SwitchOn`
  (if (`self.CanBeSwitched`)
    (`|ExecutionSequence`
      (:`then_0`
        (for _array_element (`self.LightsToSwitch`)
          (`/Engine/EditorBlueprintResources/StandardMacros.IsValid` _array_element
            (:`Is Valid`
              (`SceneComponent.SetVisibility` (`Light.LightComponent` _array_element) true false))))
        (set `self.IsOn` true))
      (:`then_1`
        (for _array_element_2 (`self.OtherSwitchesForSameLights`)
          (`/Engine/EditorBlueprintResources/StandardMacros.IsValid` _array_element_2
            (:`Is Valid`
              (set `/Game/BP/Interactive/BP_LightSwitch.IsOn` true _array_element_2))))))))

(event `SwitchOff`
  (if (`self.CanBeSwitched`)
    (`|ExecutionSequence`
      (:`then_0`
        (for _array_element (`self.LightsToSwitch`)
          (`/Engine/EditorBlueprintResources/StandardMacros.IsValid` _array_element
            (:`Is Valid`
              (`SceneComponent.SetVisibility` (`Light.LightComponent` _array_element) false false))))
        (set `self.IsOn` false))
      (:`then_1`
        (for _array_element_2 (`self.OtherSwitchesForSameLights`)
          (`/Engine/EditorBlueprintResources/StandardMacros.IsValid` _array_element_2
            (:`Is Valid`
              (set `/Game/BP/Interactive/BP_LightSwitch.IsOn` false _array_element_2))))))))

(event `self.Interaction`
  (if (`self.IsOn`)
    (`self.SwitchOff`)
    (else
      (`self.SwitchOn`))))

(fn `UserConstructionScript`
  (`parent.UserConstructionScript`))