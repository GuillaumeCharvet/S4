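; BP_Interactive is a base Blueprint for objects the player can select and interact with.
; A RaycastTrigger overlap with BP_Player sets HasToRaycast on the player controller, so raycasting is flagged only while the player is nearby.
; Interaction caches the controller if missing, then runs OnUnselected, which removes the InteractUI and clears SelectedObject.
; OnSelected is left empty.
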(event `OnSelected`)

(event `OnUnselected`
  (`/Engine/EditorBlueprintResources/StandardMacros.IsValid` (`self.PlayerController`)
    (:`Is Valid`
      (`Widget.RemoveFromParent` (`/Game/BP/Manager/BP_PC_MainPlayerController.InteractUI` (`self.PlayerController`)))
      (`/Engine/EditorBlueprintResources/StandardMacros.IsValid` (`/Game/BP/Manager/BP_PC_MainPlayerController.SelectedObject` (`self.PlayerController`))
        (:`Is Valid`
          (set `/Game/BP/Manager/BP_PC_MainPlayerController.SelectedObject` null (`self.PlayerController`)))))))

(event `Interaction`
  (`|ExecutionSequence`
    (:`then_0`
      (`/Engine/EditorBlueprintResources/StandardMacros.IsValid` (`self.PlayerController`)
        (:`Is Not Valid`
          (set `self.PlayerController` (`/Game/BP/FunctionLibraries/BP_FL_Getters.GetMyController`)))))
    (:`then_1`
      (`self.OnUnselected`))))

(event `self.RaycastTrigger.OnComponentBeginOverlap`
  (params (OverlappedComponent :type "PrimitiveComponent Object Reference") (OtherActor :type "Actor Object Reference") (OtherComp :type "PrimitiveComponent Object Reference") (OtherBodyIndex :type Integer) (bFromSweep :type Boolean) (SweepResult :type "HitResult Structure (by ref)"))
  (cast `/Game/BP/Character/BP_Player` OtherActor)
  (set `/Game/BP/Manager/BP_PC_MainPlayerController.HasToRaycast` true (`/Game/BP/FunctionLibraries/BP_FL_Getters.GetMyController`)))

(event `self.RaycastTrigger.OnComponentEndOverlap`
  (params (OverlappedComponent :type "PrimitiveComponent Object Reference") (OtherActor :type "Actor Object Reference") (OtherComp :type "PrimitiveComponent Object Reference") (OtherBodyIndex :type Integer))
  (cast `/Game/BP/Character/BP_Player` OtherActor)
  (set `/Game/BP/Manager/BP_PC_MainPlayerController.HasToRaycast` false (`/Game/BP/FunctionLibraries/BP_FL_Getters.GetMyController`)))

(fn `UserConstructionScript`)