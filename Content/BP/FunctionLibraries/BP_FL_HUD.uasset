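; Blueprint function library of HUD helpers for showing and clearing subtitles and info text.
; Each function gets the controller through GetMyController and forwards the call to its InteractUI.
; Subtitles are formatted with the talking character's enum name before the sentence and passed on with a duration, while info text is passed through unchanged.
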(fn `CallInfos`
  (params (Info :type Text :default "NSLOCTEXT(\"[A8C3495F4A529C5233EB07ABCE56BE3E]\", \"0784133643A14CEFDE219590E6350516\", \"DFAULT TEXT\")"))
  (locals (ShownText :type Text))
  (bind _output_get (set `local.ShownText` Info))
  (`/Game/BP/UI/WBP_InteractTo.EditInfosText` (`/Game/BP/Manager/BP_PC_MainPlayerController.InteractUI` (`/Game/BP/FunctionLibraries/BP_FL_Getters.GetMyController` null)) _output_get))

(fn `CallSubtitles`
  (params (Sentence :type Text :default "NSLOCTEXT(\"[A8C3495F4A529C5233EB07ABCE56BE3E]\", \"0784133643A14CEFDE219590E6350516\", \"DFAULT TEXT\")") (Duration :type "Float (double-precision)" :default 5.0) (TalkingCharacter :type "/Game/BP/Enum/BP_E_Characters Enum" :default "NewEnumerator0"))
  (locals (ShownText :type Text))
  (set `local.ShownText` (`|FormatText` "- {Character} -  \n{Sentence}" (`|GetEnumeratorNameAsString` TalkingCharacter) Sentence))
  (`/Game/BP/UI/WBP_InteractTo.Edit Subtitles Text` (`/Game/BP/Manager/BP_PC_MainPlayerController.InteractUI` (`/Game/BP/FunctionLibraries/BP_FL_Getters.GetMyController` null)) (`local.ShownText`) Duration))

(fn `RemoveInfos`
  (locals (ShownText :type Text))
  (`/Game/BP/UI/WBP_InteractTo.HideInfos` (`/Game/BP/Manager/BP_PC_MainPlayerController.InteractUI` (`/Game/BP/FunctionLibraries/BP_FL_Getters.GetMyController` null))))

(fn `RemoveSubtitles`
  (locals (ShownText :type Text))
  (`/Game/BP/UI/WBP_InteractTo.DisabledSubtitle` (`/Game/BP/Manager/BP_PC_MainPlayerController.InteractUI` (`/Game/BP/FunctionLibraries/BP_FL_Getters.GetMyController` null))))