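; BP_MyCaca is an actor that chains LaunchAnim calls to other BP_MyCaca instances by ID.
; Proces stores the incoming Id as IDLaunchedWhenFinished, and LaunchAnim searches all instances to call LaunchAnim on those whose MyID matches, with no animation or delay in the graph.
; A Box overlap prints the actor's MyID.
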(event `Proces`
  (params (NewParam :type "/Game/Trash/Struct_MyAsset Structure"))
  (set `self.ID_LaunchedWhenFinished` (`.Id_2_287499564945BB21678A7888AD2280EF` (break `/Game/Trash/Struct_MyAsset` NewParam))))

(event `LaunchAnim`
  (bind _outactors (`GameplayStatics.GetAllActorsOfClass` "BP_MyCaca_C"))
  (for _array_element _outactors
    (if (`KismetStringLibrary.EqualEqual_StrStr` (`/Game/Trash/BP_MyCaca.MyID` _array_element) (`self.ID_LaunchedWhenFinished`))
      (`self.LaunchAnim` _array_element))))

(event `self.Box.OnComponentBeginOverlap`
  (params (OverlappedComponent :type "PrimitiveComponent Object Reference") (OtherActor :type "Actor Object Reference") (OtherComp :type "PrimitiveComponent Object Reference") (OtherBodyIndex :type Integer) (bFromSweep :type Boolean) (SweepResult :type "HitResult Structure (by ref)"))
  (`KismetSystemLibrary.PrintString` (`self.MyID`)))

(fn `UserConstructionScript`)